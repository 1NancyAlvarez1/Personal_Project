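; BP_Door is a key-locked door actor that swings open and closed on interaction once HasKey is set.
; Interact alternates through a FlipFlop between playing and reversing a timeline that lerps the left door mesh's yaw for a smooth swing.
; A PickUpKey event sets HasKey, and any actor overlap briefly shows a W_INeed widget, whether or not the key is held.
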(event `self.ReceiveActorBeginOverlap`
  (params (OtherActor :type "Actor Object Reference"))
  (bind _returnvalue (`|CreateWidget` "/Game/Widgets/W_INeed.W_INeed_C"))
  (`UserWidget.AddToViewport` _returnvalue 0)
  (`KismetSystemLibrary.Delay` 3.0)
  (`Widget.RemoveFromParent` _returnvalue))

(event `/Game/Blueprints/BP_Door1.Pick Up Key`
  (set `self.Has Key?` true))

(event `/Game/Blueprints/BP_Interact.Interact`
  (if (`self.Has Key?`)
    (`/Engine/EditorBlueprintResources/StandardMacros.FlipFlop`
      (:`A`
        (bind (_direction _door_track) (`Timeline|Door Timeline` :!label _label)
          (:`Update`
            (`SceneComponent.K2_SetRelativeRotation` (`self.SM_WorkplaceSet08DoorLeft`) (`KismetMathLibrary.MakeRotator` 0.0 0.0 (`KismetMathLibrary.Lerp` 0.0 110.0 _door_track)) false false))))
      (:`B`
        (goto _label :!via `Reverse`)))))

(fn `UserConstructionScript`)